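; BP_ConsumableItem is an equippable combat-system item with a limited bag count that is spent on use.
; Equipping registers it as the owner's BP_CombatComponent item, and unequipping clears that slot.
; It supplies use montages, remaining count and whether enough remain to use.
; Consuming subtracts the per-use amount, floored at zero, and calls the component's item-changed notification, with an empty branch for depletion.
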(fn `GetRemainingItemsCount`
  (returns (NumberInBagpack :type Integer) (`bCanUse?` :type Boolean))
  (bind _numberinbagpack (`self.NumberInBagpack`))
  (return _numberinbagpack (>= _numberinbagpack (`self.NumberOfUsed`))))

(fn `GetUseItemMontages`
  (returns (UseItemMontages :type "Array of AnimMontage Object Reference"))
  (return (`self.UseItemMontages`)))

(fn `OnEquipped`
  (`parent.OnEquipped`)
  (`/Game/CombatSystem/Blueprints/Components/BP_CombatComponent.SetItem` (`self.GetComponentByClass` (`self.GetOwner`) "/Game/CombatSystem/Blueprints/Components/BP_CombatComponent.BP_CombatComponent_C") self))

(fn `OnItemConsumed`
  (bind _returnvalue (`self.GetComponentByClass` (`self.GetOwner`) "/Game/CombatSystem/Blueprints/Components/BP_CombatComponent.BP_CombatComponent_C"))
  (bind _returnvalue_2 (- (`self.NumberInBagpack`) (`self.NumberOfUsed`)))
  (bind _output_get (set `self.NumberInBagpack` (`KismetMathLibrary.Clamp` _returnvalue_2 0 _returnvalue_2)))
  (`/Game/CombatSystem/Blueprints/Components/BP_CombatComponent.OnItemChanged` _returnvalue (`/Game/CombatSystem/Blueprints/Components/BP_CombatComponent.GetItem` _returnvalue))
  (if (<= _output_get 0)
    _))

(fn `OnUnequipped`
  (`parent.OnUnequipped`)
  (`/Game/CombatSystem/Blueprints/Components/BP_CombatComponent.SetItem` (`self.GetComponentByClass` (`self.GetOwner`) "/Game/CombatSystem/Blueprints/Components/BP_CombatComponent.BP_CombatComponent_C") null))

(fn `UserConstructionScript`
  (`parent.UserConstructionScript`))