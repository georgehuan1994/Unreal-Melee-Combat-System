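; ModifyStat_AN is an anim notify that changes one of the owner's stats at a set point in an animation.
; It casts the mesh owner to BP_CombatCharacter_Base and applies the configured stat type, delta and regeneration flag through its BP_StatsComponent.
; When flagged as item consumption and set to the enum's NewEnumerator0 stat, it instead sends the owner a ConsumeItem message, leaving the stat untouched.
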(fn `Received_Notify`
  (params (MeshComp :type "SkeletalMeshComponent Object Reference") (Animation :type "AnimSequenceBase Object Reference") (EventReference :type "AnimNotifyEventReference Structure (by ref)"))
  (returns (ReturnValue :type Boolean))
  (bind _returnvalue (`ActorComponent.GetOwner` MeshComp))
  (if (and (`self.bIsCousumeItem?`) (`|EnumEquality` (`self.StatType`) "NewEnumerator0"))
    (message `/Game/CombatSystem/Blueprints/Interfaces/Combat_BPI.ConsumeItem` _returnvalue)
    (return true)
    (else
      (bind _asbp_combat_character_base (cast `/Game/CombatSystem/Blueprints/BP_CombatCharacter_Base` _returnvalue))
      (`/Game/CombatSystem/Blueprints/Components/BP_StatsComponent.ModifyCurrentStatValue` (`Actor.GetComponentByClass` _asbp_combat_character_base "/Game/CombatSystem/Blueprints/Components/BP_StatsComponent.BP_StatsComponent_C") (`self.StatType`) (`self.DeltaValue`) (`self.bShouldRegenerate?`))
      (return true))))