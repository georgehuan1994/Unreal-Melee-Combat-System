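; BP_HealthPotion is a consumable item in the combat system that restores a portion of its owner's health.
; On consumption it runs the parent behavior, then finds the owner's BP_StatsComponent and adds 30% of that stat's maximum to its current value, with the regeneration flag off.
; All other logic comes from the parent class, as the event graph holds only disabled default events.
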(fn `OnItemConsumed`
  (bind _returnvalue (`self.GetComponentByClass` (`self.GetOwner`) "/Game/CombatSystem/Blueprints/Components/BP_StatsComponent.BP_StatsComponent_C"))
  (`parent.OnItemConsumed`)
  (`/Game/CombatSystem/Blueprints/Components/BP_StatsComponent.ModifyCurrentStatValue` _returnvalue "NewEnumerator1" (* (`/Game/CombatSystem/Blueprints/Components/BP_StatsComponent.GetMaxStatValue` _returnvalue "NewEnumerator1") 0.3) false))

(fn `UserConstructionScript`
  (`parent.UserConstructionScript`))