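; Actor component that stores and manages a character's stats for the combat system, keyed by a stat enum.
; InitializeStats fills the CurrentStats map from the BaseValue of each BaseStats entry.
; ModifyCurrentStatValue adds a delta and clamps the result between zero and that stat's MaxValue, then writes it through SetCurrentStatValue, which also prints each change.
; Getters expose current, base and max values; nothing in the component calls InitializeStats itself.
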(fn `GetBaseStatValue`
  (params (Stat :type "/Game/CombatSystem/Blueprints/Enums/E_Stats Enum" :default "NewEnumerator0"))
  (returns (`Base Value` :type "Float (double-precision)"))
  (return (break `/Game/CombatSystem/Blueprints/Structs/F_BaseStat` (`BlueprintMapLibrary.Map_Find` (`self.BaseStats`) Stat))))

(fn `GetCurrentStatValue`
  (params (Stat :type "/Game/CombatSystem/Blueprints/Enums/E_Stats Enum" :default "NewEnumerator0"))
  (returns (Value :type "Float (double-precision)"))
  (return (`BlueprintMapLibrary.Map_Find` (`self.CurrentStats`) Stat)))

(fn `GetMaxStatValue`
  (params (Stat :type "/Game/CombatSystem/Blueprints/Enums/E_Stats Enum" :default "NewEnumerator0"))
  (returns (`Max Value` :type "Float (double-precision)"))
  (return (`.MaxValue_4_05C3297A468FDB41CF9899ACF8056038` (break `/Game/CombatSystem/Blueprints/Structs/F_BaseStat` (`BlueprintMapLibrary.Map_Find` (`self.BaseStats`) Stat)))))

(fn `InitializeStats`
  (bind _keys (`BlueprintMapLibrary.Map_Keys` (`self.BaseStats`)))
  (for _array_element _keys
    (`self.SetCurrentStatValue` _array_element (break `/Game/CombatSystem/Blueprints/Structs/F_BaseStat` (`BlueprintMapLibrary.Map_Find` (`self.BaseStats`) _array_element)))))

(fn `ModifyCurrentStatValue`
  (params (Stat :type "/Game/CombatSystem/Blueprints/Enums/E_Stats Enum" :default "NewEnumerator0") (NewValue :type "Float (double-precision)"))
  (locals (TempValue :type "Float (double-precision)"))
  (if (!= NewValue 0.0)
    (bind _output_get (set `local.TempValue` (+ (`self.GetCurrentStatValue` Stat) NewValue)))
    (bind _output_get_2 (set `local.TempValue` (`KismetMathLibrary.FClamp` _output_get 0.0 (`self.GetMaxStatValue` Stat))))
    (`self.SetCurrentStatValue` Stat _output_get_2)))

(fn `SetCurrentStatValue`
  (params (Stat :type "/Game/CombatSystem/Blueprints/Enums/E_Stats Enum" :default "NewEnumerator0") (NewValue :type "Float (double-precision)"))
  (`BlueprintMapLibrary.Map_Add` (`self.CurrentStats`) Stat NewValue)
  (`KismetSystemLibrary.PrintString` (`KismetStringLibrary.Concat_StrStr` (`|GetEnumeratorNameAsString` Stat) " been set to " (`KismetStringLibrary.Conv_DoubleToString` NewValue))))