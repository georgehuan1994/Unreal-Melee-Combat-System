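; Boss variant of the humanoid enemy that starts equipped and shows a boss health bar while targeted.
; BeginPlay initializes StatsComponent, then spawns and equips each starting armor piece, also spawning and equipping the starting weapon on every pass of that loop.
; OnTargeted creates a WB_BossInfo widget bound to StatsComponent when targeting begins and removes it from the viewport when targeting ends.
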(event `self.ReceiveBeginPlay`
  (`parent.ReceiveBeginPlay`)
  (`/Game/CombatSystem/Blueprints/Components/BP_StatsComponent.InitializeStats` (`self.StatsComponent`))
  (for _array_element (`self.Starting Armor`)
    (bind _returnvalue (`|SpawnActorFromClass` _array_element (`self.GetTransform`) "Undefined" "OverrideRootScale" self self))
    (`/Game/CombatSystem/Blueprints/Actors/BP_BaseEquippable.OnEquipped` _returnvalue)
    (bind _returnvalue_2 (`|SpawnActorFromClass` (`self.StartingWeapon`) (`self.GetTransform`) "Undefined" "OverrideRootScale" self null))
    (`/Game/CombatSystem/Blueprints/Actors/BP_BaseEquippable.OnEquipped` _returnvalue_2)))

(event `/Game/CombatSystem/Blueprints/Interfaces/Targeting_BPI.OnTargeted`
  (params (`bIsTargeted?` :type Boolean))
  (`parent.OnTargeted` `bIsTargeted?`)
  (if `bIsTargeted?`
    (bind _returnvalue (`|CreateWidget` "/Game/CombatSystem/UI/WB_BossInfo.WB_BossInfo_C"))
    (bind _output_get (set `self.BossInfoWidget` _returnvalue))
    (`UserWidget.AddToViewport` _output_get 0)
    (`/Game/CombatSystem/UI/WB_HealthBar.Initialize` (`/Game/CombatSystem/UI/WB_BossInfo.WB_BossHealthBar` (`self.BossInfoWidget`)) (`self.StatsComponent`))
    (else
      (`GameViewportSubsystem.RemoveWidget` (subsystem `GameViewportSubsystem`) (`self.BossInfoWidget`)))))

(fn `UserConstructionScript`
  (`parent.UserConstructionScript`))