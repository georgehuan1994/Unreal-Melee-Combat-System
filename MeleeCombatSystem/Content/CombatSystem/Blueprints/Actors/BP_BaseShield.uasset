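; BP_BaseShield is the base shield item of the combat system, handling how a shield attaches to and registers with its owner.
; On equip it attaches to its socket, caches the owner's combat and state manager components, and registers itself as the shield weapon.
; It also points its collision component at the item's static mesh, ignoring the owner.
; Unequipping runs the parent logic, then clears the combat component's shield reference.
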(fn `OnEquipped`
  (`self.SetIsEquipped` false)
  (`self.AttachActor` (`self.Attach Socket Name`))
  (set `self.BP_CombatComponent` (`self.GetComponentByClass` (`self.GetOwner`) "/Game/CombatSystem/Blueprints/Components/BP_CombatComponent.BP_CombatComponent_C"))
  (set `self.BP_StateManagerComponent` (`self.GetComponentByClass` (`self.GetOwner`) "/Game/CombatSystem/Blueprints/Components/BP_StateManagerComponent.BP_StateManagerComponent_C"))
  (`/Game/CombatSystem/Blueprints/Components/BP_CombatComponent.SetShieldWeapon` (`self.BP_CombatComponent`) self)
  (`/Game/CombatSystem/Blueprints/Components/BP_CollisionComponent.SetCollisionMeshComponent` (`self.BP_MainCollisionComponent`) (`self.ItemStaticMesh`))
  (`/Game/CombatSystem/Blueprints/Components/BP_CollisionComponent.AddIgnoreActor` (`self.BP_MainCollisionComponent`) (`self.GetOwner`)))

(fn `OnUnequipped`
  (`parent.OnUnequipped`)
  (`/Game/CombatSystem/Blueprints/Components/BP_CombatComponent.SetShieldWeapon` (`self.BP_CombatComponent`) null))

(fn `UserConstructionScript`
  (`parent.UserConstructionScript`))