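; BP_MasterAI is an AI blueprint in the combat system that manages overhead health bar and lock-on indicators.
; On BeginPlay it creates a WB_HealthBar for the first player controller, bound to its own StatsComponent rather than the player's, and assigns it to HealthBarWidget.
; OnTargeted shows or hides the lock-on widget with the targeting state, showing the health bar only when ShowHeadHealthBar is also enabled.
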(event `self.ReceiveBeginPlay`
  (`parent.ReceiveBeginPlay`)
  (bind _returnvalue (`|CreateWidget` "/Game/CombatSystem/UI/WB_HealthBar.WB_HealthBar_C" (`GameplayStatics.GetPlayerController` 0) (`self.StatsComponent`) false))
  (`WidgetComponent.SetWidget` (`self.HealthBarWidget`) _returnvalue))

(event `/Game/CombatSystem/Blueprints/Interfaces/Targeting_BPI.OnTargeted`
  (params (`bIsTargeted?` :type Boolean))
  (`SceneComponent.SetVisibility` (`self.LockOnWidget`) `bIsTargeted?` false)
  (`SceneComponent.SetVisibility` (`self.HealthBarWidget`) (and (`self.bShowHeadHealthBar?`) `bIsTargeted?`) false))

(fn `UserConstructionScript`
  (`parent.UserConstructionScript`))