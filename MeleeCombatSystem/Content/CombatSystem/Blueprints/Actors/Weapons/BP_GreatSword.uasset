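; Great sword weapon Blueprint that handles the landing phase of its owner's special attack.
; When OnOwnerLanded receives the Special Attack gameplay tag, it plays an end montage on the owning Character's mesh and zeroes movement velocity.
; BeginPlay, overlap and Tick are disabled stubs, and the construction script only calls its parent.
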(event `/Game/CombatSystem/Blueprints/Interfaces/Weapon_BPI.OnOwnerLanded`
  (params (InGameplayTag :type "GameplayTag Structure"))
  (bind _ascharacter (cast `Character` (`self.GetOwner`) :!pure true))
  (`|SwitchGameplayTag` InGameplayTag
    (:`Character.Action.Attack.Special Attack`
      (`AnimInstance.Montage_Play` (`SkeletalMeshComponent.GetAnimInstance` (`Character.Mesh` _ascharacter)) "/Game/Characters/Mannequin_UE4/Animations/GreatSword/Battle/Inplace/GreatSword_SPAttack2_End_Montage.GreatSword_SPAttack2_End_Montage" 1.0 "Duration" 0.0 true)
      (set `MovementComponent.Velocity` (0.0 0.0 0.0) (`Pawn.GetMovementComponent` _ascharacter)))))

(fn `GetOwnedGameplayTags`
  (returns (ReturnValue :type "GameplayTagContainer Structure"))
  (return))

(fn `UserConstructionScript`
  (`parent.UserConstructionScript`))