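; BP_CombatDummy is a targetable combat dummy for the combat system.
; On BeginPlay it initializes its stats component, then spawns and equips each starting armor piece, spawning and equipping the starting weapon inside that same loop.
; The targeting callback toggles a lock-on widget's visibility.
; It reports itself as targetable unless its state manager component is in the Dead state.
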(event `self.ReceiveBeginPlay`
  (`/Game/CombatSystem/Blueprints/Components/BP_StatsComponent.InitializeStats` (`self.StatsComponent`))
  (for _array_element (`self.StartingArmor`)
    (bind _returnvalue (`|SpawnActorFromClass` _array_element (`self.GetTransform`) "Undefined" "OverrideRootScale" self self))
    (`/Game/CombatSystem/Blueprints/Actors/BP_BaseEquippable.OnEquipped` _returnvalue)
    (bind _returnvalue_2 (`|SpawnActorFromClass` (`self.StartingWeapon`) (`self.GetTransform`) "Undefined" "OverrideRootScale" self null))
    (`/Game/CombatSystem/Blueprints/Actors/BP_BaseEquippable.OnEquipped` _returnvalue_2)))

(event `/Game/CombatSystem/Blueprints/Interfaces/Targeting_BPI.OnTargeted`
  (params (`bIsTargeted?` :type Boolean))
  (`SceneComponent.SetVisibility` (`self.LockOnWidget`) `bIsTargeted?` false))

(fn `CanBeTargeted?`
  (returns (ReturnValue :type Boolean))
  (return (not (`/Game/CombatSystem/Blueprints/Components/BP_StateManagerComponent.IsCurrentStateEqualToAny?` (`self.StateManagerComponent`) (struct :`GameplayTags` (struct :`(TagName` "Character.State.Dead")))))))

(fn `UserConstructionScript`
  (`parent.UserConstructionScript`))