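; Base weapon Blueprint for the combat system, holding per-action montages, stat costs and damage.
; On equip it registers as the owner's main weapon, sends its combat type to the AnimInstance and sets up its collision component to ignore the owner.
; Collision hits apply point damage to receptive actors, scaled by the state manager's current action.
; Montages are selected by action gameplay tag, and the mesh can switch to physics simulation.
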(event `self.BP_CollisionComponent.OnHit`
  (params (HitResult :type "HitResult Structure"))
  (bind (_bblockinghit _binitialoverlap _time _distance _location _impactpoint _normal _impactnormal _physmat _hitactor) (`GameplayStatics.BreakHitResult` HitResult))
  (bind _returnvalue (message `/Game/CombatSystem/Blueprints/Interfaces/Combat_BPI.CanRecieveDamage` _hitactor))
  (if _returnvalue
    (`GameplayStatics.ApplyPointDamage` _hitactor (`self.GetDamage`) (`self.GetActorForwardVector` (`self.GetOwner`)) HitResult (`self.GetInstigatorController`) self)))

(event `SimulateWeaponPhysics`
  (`PrimitiveComponent.SetCollisionProfileName` (`self.GetItemMesh`) "PhysicsActor" true)
  (`PrimitiveComponent.SetSimulatePhysics` (`self.GetItemMesh`) true))

(fn `GetActionMontages`
  (params (CharacterAction :type "GameplayTag Structure"))
  (returns (Montages :type "Array of AnimMontage Object Reference"))
  (`|SwitchGameplayTag` CharacterAction
    (:`Character.Action.Attack.Light Attack`
      (return (`self.LightAttackMontages`)))
    (:`Character.Action.Attack.Heavy Attack`
      (return (`self.HeavyAttackMontages`)))
    (:`Character.Action.Attack.Charged Attack`
      (return (`self.ChargedAttackMontages`)))
    (:`Character.Action.Attack.Falling Attack`
      (return (`self.FallingAttackMontages`)))
    (:`Character.Action.Attack.Sprinting Attack`
      (return (`self.SprintingAttackMontages`)))
    (:`Character.Action.Dodge`
      (return (`self.DodgeMontages`)))
    (:`Character.Action.Enter Combat`
      (return (`|MakeArray` (`self.EnterCombat`))))
    (:`Character.Action.Exit Conbat`
      (return (`|MakeArray` (`self.ExitCombat`))))))

(fn `GetDamage`
  (returns (ReturnValue :type "Float (double-precision)"))
  (bind _bp_statemanagercomponent (`self.BP_StateManagerComponent`)
    (:`then`
      (bind _value (`BlueprintMapLibrary.Map_Find` (`self.ActionDamageMultiplier`) (`/Game/CombatSystem/Blueprints/Components/BP_StateManagerComponent.GetCurrentAction` _bp_statemanagercomponent)))
      (return (* (`self.Damage`) (`KismetMathLibrary.FClamp` _value 1.0 _value))))
    (:`else`
      (return (`self.Damage`)))))

(fn `GetStatCostForAction`
  (returns (Value :type "Float (double-precision)"))
  (bind _bp_statemanagercomponent (`self.BP_StateManagerComponent`)
    (:`then`
      (return (`BlueprintMapLibrary.Map_Find` (`self.ActionStatCost`) (`/Game/CombatSystem/Blueprints/Components/BP_StateManagerComponent.GetCurrentAction` _bp_statemanagercomponent))))
    (:`else`
      (return 0.0))))

(fn `OnEquipped`
  (`parent.OnEquipped`)
  (`self.SetIsEquipped` true)
  (set `self.BP_CombatComponent` (`self.GetComponentByClass` (`self.GetOwner`) "/Game/CombatSystem/Blueprints/Components/BP_CombatComponent.BP_CombatComponent_C"))
  (set `self.BP_StateManagerComponent` (`self.GetComponentByClass` (`self.GetOwner`) "/Game/CombatSystem/Blueprints/Components/BP_StateManagerComponent.BP_StateManagerComponent_C"))
  (`/Game/CombatSystem/Blueprints/Components/BP_CombatComponent.SetMainWeapon` (`self.BP_CombatComponent`) self)
  (message `/Game/CombatSystem/Blueprints/Interfaces/AnimInstance_BPI.UpdateCombatType` (`SkeletalMeshComponent.GetAnimInstance` (`Character.Mesh` (cast `Character` (`self.GetOwner`) :!pure true))) (`self.CombatType`))
  (`/Game/CombatSystem/Blueprints/Components/BP_CollisionComponent.SetCollisionMeshComponent` (`self.BP_CollisionComponent`) (`self.ItemStaticMesh`))
  (`/Game/CombatSystem/Blueprints/Components/BP_CollisionComponent.AddIgnoreActor` (`self.BP_CollisionComponent`) (`self.GetOwner`)))

(fn `UserConstructionScript`
  (`parent.UserConstructionScript`))