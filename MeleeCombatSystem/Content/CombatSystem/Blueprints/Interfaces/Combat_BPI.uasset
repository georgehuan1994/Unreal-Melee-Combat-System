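; Combat_BPI is a Blueprint interface that defines the contract between combat-capable actors and the systems that drive them.
; It declares calls to perform attacks, actions and item use, returning success and a duration, with attacks flagging whether AI triggered them.
; Further functions continue or reset attacks and combat, consume items, toggle movement, and query desired rotation, speed mode and whether damage can be received.
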(fn `CanMove`
  (params (`bCanMove?` :type Boolean)))

(fn `CanRecieveDamage`
  (returns (ReturnValue :type Boolean))
  (return false))

(fn `ConsumeItem`)

(fn `ContinueAttack`)

(fn `GetDesireRotation`
  (returns (NewRotator :type "Rotator Structure"))
  (return))

(fn `GetSpeedMode`
  (returns (ReturnValue :type "/Game/CombatSystem/Blueprints/Enums/E_MovementSpeedMode Enum"))
  (return "NewEnumerator0"))

(fn `PerformAction`
  (params (CharacterState :type "GameplayTag Structure") (CharacterAction :type "GameplayTag Structure") (MontageIndex :type Integer) (`bRandomIndex?` :type Boolean))
  (returns (`bSuccess?` :type Boolean) (ActionDuration :type "Float (double-precision)"))
  (return false 0.0))

(fn `PerformAttack`
  (params (AttackType :type "GameplayTag Structure") (AttackIndex :type Integer) (`bRandomIndex?` :type Boolean) (`bIsCalledByAI?` :type Boolean))
  (returns (`bSuccess?` :type Boolean) (AttackDuration :type "Float (double-precision)"))
  (return false 0.0))

(fn `PerformUseItem`
  (params (CharacterState :type "GameplayTag Structure") (CharacterAction :type "GameplayTag Structure") (MontagePlayRate :type "Float (double-precision)" :default 1.0) (MontageIndex :type Integer) (`bRandomIndex?` :type Boolean))
  (returns (`bSuccess?` :type Boolean) (ActionDuration :type "Float (double-precision)"))
  (return false 0.0))

(fn `ResetAttack`)

(fn `ResetCombat`)