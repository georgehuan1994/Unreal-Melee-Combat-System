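; Base AI controller for combat AI that runs the possessed BP_MasterAI's behavior tree and feeds its blackboard.
; On possess it binds to the pawn's CombatComponent toggle event to mirror combat state into bCombatEnable.
; Perception updates treat stimulus index 0 as sight and 1 as damage, setting Target only to actors tagged Character.Player.
; Failed or non-player sight stimuli clear Target, while damage can only set it.
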(event `self.ReceivePossess`
  (params (PossessedPawn :type "Pawn Object Reference"))
  (bind _asbp_master_ai (cast `/Game/CombatSystem/Blueprints/AI/BP_MasterAI` PossessedPawn))
  (bind _output_get (set `self.Master AI` _asbp_master_ai))
  (add `/Game/CombatSystem/Blueprints/Components/BP_CombatComponent.OnToggleCombat` (`/Game/CombatSystem/Blueprints/BP_CombatCharacter_UE4.CombatComponent` (`self.Master AI`)) (delegate `OnToggleCombat AI`))
  (`self.RunBehaviorTree` (`/Game/CombatSystem/Blueprints/AI/BP_MasterAI.Behavior Tree` _output_get)))

(event `OnToggleCombat AI`
  (params (`bCombatEnable?` :type Boolean))
  (`BlackboardComponent.SetValueAsBool` (`self.Blackboard`) "bCombatEnable" `bCombatEnable?`))

(event `self.AIPerception.OnPerceptionUpdated`
  (params (UpdatedActors :type "Array of Actor Object Reference (by ref)"))
  (`self.UpdatePerception` UpdatedActors))

(fn `SetTargetActor`
  (params (NewTargetActor :type "Actor Object Reference"))
  (`BlackboardComponent.SetValueAsObject` (`self.Blackboard`) "Target" NewTargetActor))

(fn `UpdatePerception`
  (params (PerceivedActors :type "Array of Actor Object Reference"))
  (locals (TheSensedActor :type "Actor Object Reference") (LastStimuli :type "AIStimulus Structure"))
  (bind (_age _expirationage _strength _stimuluslocation _receiverlocation _tag _bsuccessfullysensed) (break `AIStimulus` (`local.LastStimuli`)))
  (for _array_element PerceivedActors
    (bind _output_get (set `local.TheSensedActor` _array_element))
    (bind _info (`AIPerceptionComponent.GetActorsPerception` (`self.AIPerception`) _output_get))
    (for (_array_element_2 _array_index) (`.LastSensedStimuli` (break `ActorPerceptionBlueprintInfo` _info))
      (set `local.LastStimuli` _array_element_2)
      (switch `int` _array_index :!pinned true ; 0: AI sight\n1: AI damage sense
        (:`0`
          (if _bsuccessfullysensed
            (bind _returnvalue (message `/Game/CombatSystem/Blueprints/Interfaces/GameplayTag_BPI.HasMatchingGameplayTag` _output_get (struct :`TagName` "Character.Player")))
            (if _returnvalue
              (`self.SetTargetActor` (`local.TheSensedActor`))
              (else
                (`self.SetTargetActor` null :!label _label)))
            (else
              (goto _label))))
        (:`1`
          (if _bsuccessfullysensed
            (bind _returnvalue_2 (message `/Game/CombatSystem/Blueprints/Interfaces/GameplayTag_BPI.HasMatchingGameplayTag` (`local.TheSensedActor`) (struct :`TagName` "Character.Player")))
            (if _returnvalue_2
              (`self.SetTargetActor` (`local.TheSensedActor`)))))))))

(fn `UserConstructionScript`)