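; CombatComponent is a component for a Character that tracks its main weapon and whether combat is enabled.
; Setting a new main weapon first unequips and destroys any valid current one, then stores the new reference.
; Changing the combat state stores the flag and passes it to the owner's mesh AnimInstance through an UpdateCombatEnabled message.
; It runs no BeginPlay or Tick logic.
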(fn `GetMainWeapon`
  (returns (MainWeapon :type "/Game/CombatSystem/Blueprints/Actors/BP_BaseWeapon Object Reference"))
  (return (`self.MainWeapon`)))

(fn `IsCombatEnable?`
  (returns (`bIsCombatEnable?` :type Boolean))
  (return (`self.bIsCombatEnable?`)))

(fn `SetCombatEnable`
  (params (`bIsCombatEnable?` :type Boolean))
  (bind _output_get (set `self.bIsCombatEnable?` `bIsCombatEnable?`))
  (message `/Game/CombatSystem/Blueprints/Interfaces/AnimInstance_BPI.UpdateCombatEnabled` (`SkeletalMeshComponent.GetAnimInstance` (`Character.Mesh` (cast `Character` (`self.GetOwner`) :!pure true))) _output_get))

(fn `SetMainWeapon`
  (params (NewWeapon :type "/Game/CombatSystem/Blueprints/Actors/BP_BaseWeapon Object Reference"))
  (`|ExecutionSequence`
    (:`then_0`
      (bind _mainweapon (`self.MainWeapon`)
        (:`then`
          (`/Game/CombatSystem/Blueprints/Actors/BP_BaseEquippable.OnUnequipped` _mainweapon)
          (`Actor.K2_DestroyActor` _mainweapon))
        (:`else`)))
    (:`then_1`
      (set `self.MainWeapon` NewWeapon))))