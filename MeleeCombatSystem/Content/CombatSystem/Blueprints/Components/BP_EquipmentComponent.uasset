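; BP_EquipmentComponent is an actor component that gives its owner a starting set of equipment.
; InitializeEquipment spawns each valid class in StartingEquipments at the owner's transform, with the owner set as Owner and as pawn Instigator.
; It then calls OnEquipped on each spawned actor and stores it in CurrentEquipments, which GetCurrentEquipments returns.
; BeginPlay and Tick are empty, and nothing in the component calls InitializeEquipment.
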(fn `GetCurrentEquipments`
  (returns (CurrentEquipments :type "Array of /Game/CombatSystem/Blueprints/Actors/BP_BaseEquippable Object Reference"))
  (return (`self.CurrentEquipments`)))

(fn `InitializeEquipment`
  (bind _returnvalue (`self.GetOwner`))
  (for _array_element (`self.StartingEquipments`)
    (if (`KismetSystemLibrary.IsValidClass` _array_element)
      (bind _returnvalue_2 (`|SpawnActorFromClass` _array_element (`Actor.GetTransform` _returnvalue) "Undefined" "OverrideRootScale" _returnvalue (cast `Pawn` _returnvalue :!pure true)))
      (`/Game/CombatSystem/Blueprints/Actors/BP_BaseEquippable.OnEquipped` _returnvalue_2)
      (`KismetArrayLibrary.Array_AddUnique` (`self.CurrentEquipments`) _returnvalue_2)))
  (return))