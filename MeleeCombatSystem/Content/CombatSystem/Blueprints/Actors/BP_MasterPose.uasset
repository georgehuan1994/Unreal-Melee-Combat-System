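; BP_MasterPose is an equippable armor actor whose skeletal mesh follows the animation of its owning Character.
; AttachActor snaps the item mesh to a socket on the character mesh and sets that mesh as its leader pose component, so both animate together.
; OnEquipped and OnUnequipped add or subtract BaseArmor through the owner's BP_StatsComponent and register or remove the item with BP_CombatComponent.
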(fn `AttachActor`
  (params (SocketName :type Name))
  (bind _itemskeletalmesh (`self.ItemSkeletalMesh`))
  (bind _mesh (`Character.Mesh` (cast `Character` (`self.GetOwner`) :!pure true)))
  (`/Engine/EditorBlueprintResources/StandardMacros.IsValid` (`SkinnedMeshComponent.SkinnedAsset` _itemskeletalmesh)
    (:`Is Valid`
      (`SceneComponent.K2_AttachToComponent` _itemskeletalmesh _mesh SocketName "SnapToTarget" "SnapToTarget" "SnapToTarget" true)
      (`SkinnedMeshComponent.SetLeaderPoseComponent` _itemskeletalmesh _mesh false false)
      (return))))

(fn `OnEquipped`
  (`parent.OnEquipped`)
  (`/Game/CombatSystem/Blueprints/Components/BP_StatsComponent.ModifyCurrentStatValue` (`self.GetComponentByClass` (`self.GetOwner`) "/Game/CombatSystem/Blueprints/Components/BP_StatsComponent.BP_StatsComponent_C") "NewEnumerator3" (`self.BaseArmor`) false)
  (`/Game/CombatSystem/Blueprints/Components/BP_CombatComponent.AddEquipment` (`self.GetComponentByClass` (`self.GetOwner`) "/Game/CombatSystem/Blueprints/Components/BP_CombatComponent.BP_CombatComponent_C") self))

(fn `OnUnequipped`
  (`parent.OnUnequipped`)
  (`/Game/CombatSystem/Blueprints/Components/BP_StatsComponent.ModifyCurrentStatValue` (`self.GetComponentByClass` (`self.GetOwner`) "/Game/CombatSystem/Blueprints/Components/BP_StatsComponent.BP_StatsComponent_C") "NewEnumerator3" (* (`self.BaseArmor`) -1.0) false)
  (`/Game/CombatSystem/Blueprints/Components/BP_CombatComponent.RemoveEquipment` (`self.GetComponentByClass` (`self.GetOwner`) "/Game/CombatSystem/Blueprints/Components/BP_CombatComponent.BP_CombatComponent_C") self))

(fn `UserConstructionScript`
  (`parent.UserConstructionScript`))