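; Base Blueprint for dual-wielded weapons in the combat system, extending a parent weapon with an off-hand mesh and a second collision component.
; On equip, it snaps the second mesh to a socket on the owning character's mesh, binds the second collision component to it and ignores the owner.
; Collision toggles per part (main or off-hand), and second-component hits feed the same OnHit handler.
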(event `self.BP_SecondCollisionComponent.OnHit`
  (params (HitResult :type "HitResult Structure"))
  (`self.On Hit` HitResult))

(fn `ActivateCollision`
  (params (CollisionPart :type "/Game/CombatSystem/Blueprints/Enums/E_CollisionPart Enum" :default "NewEnumerator0"))
  (switch `/Game/CombatSystem/Blueprints/Enums/E_CollisionPart` CollisionPart
    (:`NewEnumerator0`
      (`/Game/CombatSystem/Blueprints/Components/BP_CollisionComponent.Activate Collision` (`self.BP_MainCollisionComponent`)))
    (:`NewEnumerator1`
      (`/Game/CombatSystem/Blueprints/Components/BP_CollisionComponent.Activate Collision` (`self.BP_SecondCollisionComponent`)))))

(fn `AttachOffHandWeapon`
  (params (Socket :type Name))
  (`SceneComponent.K2_AttachToComponent` (`self.ItemStaticMesh2`) (`Character.Mesh` (cast `Character` (`self.GetOwner`) :!pure true)) Socket "SnapToTarget" "SnapToTarget" "SnapToTarget" true))

(fn `DeactivateCollision`
  (params (CollisionPart :type "/Game/CombatSystem/Blueprints/Enums/E_CollisionPart Enum" :default "NewEnumerator0"))
  (switch `/Game/CombatSystem/Blueprints/Enums/E_CollisionPart` CollisionPart
    (:`NewEnumerator0`
      (`/Game/CombatSystem/Blueprints/Components/BP_CollisionComponent.Deactivate Collision` (`self.BP_MainCollisionComponent`)))
    (:`NewEnumerator1`
      (`/Game/CombatSystem/Blueprints/Components/BP_CollisionComponent.Deactivate Collision` (`self.BP_SecondCollisionComponent`)))))

(fn `OnEquipped`
  (`parent.OnEquipped`)
  (`/Game/CombatSystem/Blueprints/Components/BP_CollisionComponent.SetCollisionMeshComponent` (`self.BP_SecondCollisionComponent`) (`self.ItemStaticMesh2`))
  (`self.AttachOffHandWeapon` (`self.AttachSocketName2`))
  (`/Game/CombatSystem/Blueprints/Components/BP_CollisionComponent.AddIgnoreActor` (`self.BP_SecondCollisionComponent`) (`self.GetOwner`)))

(fn `UserConstructionScript`
  (`parent.UserConstructionScript`))